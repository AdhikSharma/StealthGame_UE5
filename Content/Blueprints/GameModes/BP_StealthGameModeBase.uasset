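; Stealth game mode Blueprint that shows the game over screen when a mission completes.
; OnMissionCompleted creates WBP_GameOverScreen, passing it the success flag, and adds it to the viewport.
; GetAllCheckpoints returns the first BP_CheckPoint matching a given index; BeginPlay only prints the result for index 1.
; A camera blend to BP_SpectatingViewpoint is present but disconnected, so it never runs.
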(event `self.ReceiveBeginPlay`
  (bind _checkpoints (`self.GetAllCheckpoints` 1))
  (`KismetSystemLibrary.PrintString` (`KismetSystemLibrary.GetDisplayName` _checkpoints) true true (struct :`G` 0.66 :`B` 1.0 :`A` 1.0) 5.0))

(event `self.OnMissionCompleted`
  (params (instigatorPawn :type "Pawn Object Reference") (missionSuccess :type Boolean))
  (`|ExecutionSequence`
    (:`then_0`
      (bind _returnvalue (`|CreateWidget` "/Game/Blueprints/Widget/WBP_GameOverScreen.WBP_GameOverScreen_C" null missionSuccess))
      (`UserWidget.AddToViewport` _returnvalue 0))))

(fn `GetAllCheckpoints`
  (params (CheckpointIndex :type Integer))
  (returns (Checkpoints :type "/Game/Blueprints/Actors/BP_CheckPoint Object Reference"))
  (bind _outactors (`GameplayStatics.GetAllActorsOfClass` "/Game/Blueprints/Actors/BP_CheckPoint.BP_CheckPoint_C"))
  (for _array_element _outactors
    (if (== (`/Game/Blueprints/Actors/BP_CheckPoint.CHeckpointIndex` _array_element) CheckpointIndex)
      (return _array_element))))

(fn `UserConstructionScript`)