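; BP_LaunchPad is a launch pad actor that flings characters and physics objects that overlap it.
; A StealthGameCharacter receives LaunchCharacter, while any other actor gets a velocity-change impulse if its root primitive simulates physics, making that impulse mass-independent.
; Both use an upward speed plus a forward speed scaled only by the X component of the mesh's forward vector, with no Y component.
; Debug strings print on the non-character path.
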(event `self.ReceiveActorBeginOverlap`
  (params (OtherActor :type "Actor Object Reference"))
  (bind _launchspeedup (`self.LaunchSpeedUp`))
  (bind _returnvalue_x (`KismetMathLibrary.BreakVector` (`SceneComponent.GetForwardVector` (`self.StaticMesh`))))
  (bind _returnvalue (* _returnvalue_x (`self.LaunchSpeedFwd`)))
  (bind _asstealth_game_character (cast `StealthGameCharacter` OtherActor)
    (:`then`
      (`Character.LaunchCharacter` _asstealth_game_character (`KismetMathLibrary.MakeVector` _returnvalue 0.0 _launchspeedup) false false))
    (:`CastFailed`
      (bind _asprimitive_component (cast `PrimitiveComponent` (`Actor.RootComponent` OtherActor)))
      (`KismetSystemLibrary.PrintString` "Got cube")
      (if (`SceneComponent.IsSimulatingPhysics` _asprimitive_component "None")
        (`KismetSystemLibrary.PrintString` "Add force")
        (`PrimitiveComponent.AddImpulse` _asprimitive_component (`KismetMathLibrary.MakeVector` _returnvalue 0.0 _launchspeedup) "None" true)))))

(fn `UserConstructionScript`)